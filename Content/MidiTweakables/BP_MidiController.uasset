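; BP_MidiController brings hardware MIDI input into the game and rebroadcasts it as Blueprint events.
; On BeginPlay it prints the input devices it finds with their IDs, then creates an input controller for the configured device ID.
; Note on, note off and control change handlers pass note, or CC number and value, to matching dispatchers, dropping channel and velocity, with optional debug printing.
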(event `self.ReceiveBeginPlay`
  (`|ExecutionSequence`
    (:`then_0`
      (`self.PrintMidiInDevices`))
    (:`then_1`
      (`self.BindMidiController` (`self.DeviceIDToBind`)))))

(event `OnMidiNoteOn`
  (params (MIDIDeviceController :type "MIDIDeviceInputController Object Reference") (Timestamp :type Integer) (Channel :type Integer) (Note :type Integer) (Velocity :type Integer))
  ;[1 1 1] print midi inputs
  (if (`self.PrintInputs`)
    (`KismetSystemLibrary.PrintString` (`KismetStringLibrary.Concat_StrStr` "NoteOn: " (`KismetStringLibrary.Conv_IntToString` Note))))
  (`self.MidiNoteOn` Note))

(event `OnMidiNoteOff`
  (params (MIDIDeviceController :type "MIDIDeviceInputController Object Reference") (Timestamp :type Integer) (Channel :type Integer) (Note :type Integer) (Velocity :type Integer))
  ;[1 1 1] print midi inputs
  (if (`self.PrintInputs`)
    (`KismetSystemLibrary.PrintString` (`KismetStringLibrary.Concat_StrStr` "NoteOff: " (`KismetStringLibrary.Conv_IntToString` Note))))
  (`self.MidiNoteOff` Note))

(event `OnMidiControlChange`
  (params (MIDIDeviceController :type "MIDIDeviceInputController Object Reference") (Timestamp :type Integer) (Channel :type Integer) (Type :type Integer) (Value :type Integer))
  ;[1 1 1] print midi inputs
  (if (`self.PrintInputs`)
    (`KismetSystemLibrary.PrintString` (`KismetStringLibrary.Concat_StrStr` "CC: " (`KismetStringLibrary.Conv_IntToString` Type) "  " (`KismetStringLibrary.Conv_IntToString` Value))))
  (`self.MidiControlChange` Type Value))

(fn `BindMidiController`
  (params (DeviceID :type Integer))
  (bind _returnvalue (`MIDIDeviceManager.CreateMIDIDeviceInputController` DeviceID))
  (bind _output_get (set `self.MidiController` _returnvalue))
  (add `MIDIDeviceInputController.OnMIDINoteOn` _output_get (`|CreateDelegate` :!event `OnMidiNoteOn`))
  (add `MIDIDeviceInputController.OnMIDINoteOff` _output_get (`|CreateDelegate` :!event `OnMidiNoteOff`))
  (add `MIDIDeviceInputController.OnMIDIControlChange` _output_get (`|CreateDelegate` :!event `OnMidiControlChange`)))

(fn `PrintMidiInDevices`
  (bind _outmididevices (`MIDIDeviceManager.FindMIDIDevices`))
  (for _array_element _outmididevices
    (bind (_deviceid _devicename _bcanreceivefrom) (break `FoundMIDIDevice` _array_element))
    (if _bcanreceivefrom
      (`KismetSystemLibrary.PrintString` (`KismetStringLibrary.Concat_StrStr` "Midi Device found: " _devicename " with ID: " (`KismetStringLibrary.Conv_IntToString` _deviceid))))))

(fn `UserConstructionScript`)